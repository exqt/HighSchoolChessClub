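; Player Blueprint for chess matches that shows the screen matching the current match state.
; On possession it binds to the ChessMatch state change, then swaps setup, play or result widgets, pushed asynchronously to the in-game UI stack and tracked for cleanup.
; The setup screen's start click applies settings and requests the match start, while the play screen receives the match.
; Unpossession clears widgets and unbinds; a debug F key returns to exploration.
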(event Custom|OnClickStart_Event_2
  (params (MatchSetting :type Chess%20Match%20Settings%20Structure))
  ;[0.15 0.15 0.15 0.5] ChessMatch 상태에 따라 해당 되는 UI 보여주기
)

(event Custom|OnClickStart_Event_3
  (params (MatchSetting :type Chess%20Match%20Settings%20Structure))
  ;[0.15 0.15 0.15 0.5] ChessMatch 상태에 따라 해당 되는 UI 보여주기
)

(event Custom|OnMatchStateChanged_Event
  (params (NewState :type EChessMatchState%20Enum :default "WaitingForPlayers"))
  (bind _managedscreenwidgets (Variables|Default|GetManagedScreenWidgets))
  (bind _managedscreenwidgets_2 (Variables|Default|GetManagedScreenWidgets))
  ;[0.15 0.15 0.15 0.5] ChessMatch 상태에 따라 해당 되는 UI 보여주기
  (for _array_element _managedscreenwidgets
    (Class|CommonActivatableWidget|DeactivateWidget _array_element))
  (Utilities|Array|Clear _managedscreenwidgets)
  (switch Utilities|FlowControl|Switch|SwitchonEChessMatchState NewState
    (:MatchSetup
      (bind _widget (|PushSoftWidgettoStackAsync "(TagName=\"UI.Stack.InGame\")" "/Game/UI/Widgets/InGame/WBP_GameSetupScreen.WBP_GameSetupScreen_C")
        (:OnSuccess
          (Utilities|Array|Add _managedscreenwidgets_2 _widget)
          (bind _aswbp_game_setup_screen (Utilities|Casting|CastToWBP_GameSetupScreen _widget))
          (EventDispatchers|AssignOnClickStart _aswbp_game_setup_screen (delegate Custom|OnClickStart_Event)))))
    (:Playing
      (bind _widget_2 (|PushSoftWidgettoStackAsync "(TagName=\"UI.Stack.InGame\")" "/Game/UI/Widgets/PlayChess/WBP_PlayChessScreen.WBP_PlayChessScreen_C")
        (:OnSuccess
          (Utilities|Array|Add _managedscreenwidgets_2 _widget_2)
          (bind _aswbp_play_chess_screen (Utilities|Casting|CastToWBP_PlayChessScreen _widget_2))
          (Default|InitChessMatch _aswbp_play_chess_screen (Class|ChessPlayer|GetChessMatch)))))
    (:Finished
      (bind _widget_3 (|PushSoftWidgettoStackAsync "(TagName=\"UI.Stack.InGame\")" "/Game/UI/Widgets/InGame/WBP_GameResultScreen.WBP_GameResultScreen_C")
        (:then
          (Utilities|Casting|CastToWBP_GameResultScreen _widget_3))
        (:OnSuccess
          (Utilities|Array|Add _managedscreenwidgets_2 _widget_3))))))

(event Custom|OnClickStart_Event_0
  (params (MatchSetting :type Chess%20Match%20Settings%20Structure))
  ;[0.15 0.15 0.15 0.5] ChessMatch 상태에 따라 해당 되는 UI 보여주기
)

(event Custom|OnClickStart_Event_1
  (params (MatchSetting :type Chess%20Match%20Settings%20Structure))
  ;[0.15 0.15 0.15 0.5] ChessMatch 상태에 따라 해당 되는 UI 보여주기
)

(event Custom|OnClickStart_Event
  (params (MatchSetting :type Chess%20Match%20Settings%20Structure))
  ;[0.15 0.15 0.15 0.5] ChessMatch 상태에 따라 해당 되는 UI 보여주기
  (Class|ChessMatch|SetMatchSettings (Class|ChessPlayer|GetChessMatch) MatchSetting)
  (Class|ChessPlayer|RequestStartMatch))

(event EventPossessed
  (params (NewController :type Controller%20Object%20Reference))
  (bind _returnvalue (Class|ChessPlayer|GetChessMatch))
  ;[0.15 0.15 0.15 0.5] ChessMatch 상태에 따라 해당 되는 UI 보여주기
  (Utilities|IsValid _returnvalue
    (:Is%20Valid
      (EventDispatchers|BindEventtoOnMatchStateChanged _returnvalue (delegate Custom|OnMatchStateChanged_Event)))))

(event EventUnpossessed
  (params (OldController :type Controller%20Object%20Reference))
  (bind _returnvalue (Class|ChessPlayer|GetChessMatch))
  (bind _managedscreenwidgets (Variables|Default|GetManagedScreenWidgets))
  ;[0.15 0.15 0.15 0.5] ChessMatch 상태에 따라 해당 되는 UI 보여주기
  ;;[0.15 0.15 0.15 0.5] Unposses시 정리
  (for _array_element _managedscreenwidgets
    (Class|CommonActivatableWidget|DeactivateWidget _array_element))
  (Utilities|Array|Clear _managedscreenwidgets)
  (Utilities|IsValid _returnvalue
    (:Is%20Valid
      (EventDispatchers|UnbindEventfromOnMatchStateChanged _returnvalue (delegate Custom|OnMatchStateChanged_Event)))))

(event Input|KeyboardEvents|DebugKeyF
  (params (Key :type Key%20Structure :default "None") (ActionValue :type Input%20Action%20Value%20Structure))
  (:Pressed
    (Class|ChessPlayer|ReturntoExploration)))

(fn ConstructionScript)