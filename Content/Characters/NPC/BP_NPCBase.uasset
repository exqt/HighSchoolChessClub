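; Base NPC character that the player can talk to and that plays chess move animations.
; Interacting sends a dialogue-start event to the AI controller's StateTree and enables look-at, which also follows dialogue subsystem state changes.
; Tick feeds the player's look-at position and the NPC state into the anim Blueprint.
; Chess moves play a montage whose notifies attach the piece to a hand socket and tween it into place, then report completion.
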(event Custom|OnDialogueActiveChanged_Event
  (params (bIsActive :type Boolean))
  ;[0.15 0.15 0.15 0.5] Dialgoue Init
  (if bIsActive
    (Variables|/Game/Characters/NPC/ABP_NPCBase.ABP_NPCBase_C|SetbEnableLookAt (Variables|Default|GetABP%20NPCBase) true)
    (else
      (Variables|/Game/Characters/NPC/ABP_NPCBase.ABP_NPCBase_C|SetbEnableLookAt (Variables|Default|GetABP%20NPCBase) false))))

(event Custom|OnDialogueActiveChanged_Event_0
  (params (bIsActive :type Boolean))
  ;[0.15 0.15 0.15 0.5] Dialgoue Init
)

(event EventInteract
  (params (Interactor :type Pawn%20Object%20Reference))
  ;[0.15 0.15 0.15 0.5] Interaction
  (bind _statetree (CallFunction|GetStateTree))
  (Gameplay|StateTree|SendStateTreeEvent _statetree (Utilities|Struct|MakeStateTreeEvent "(TagName=\"NPCEvent.Dialogue.Start\")") :!class /Script/GameplayStateTreeModule.StateTreeComponent)
  (Variables|/Game/Characters/NPC/ABP_NPCBase.ABP_NPCBase_C|SetbEnableLookAt (Variables|Default|GetABP%20NPCBase) true))

(event EventBeginPlay
  (Utilities|FlowControl|Sequence
    (:then_0
      ;[0.15 0.15 0.15 0.5] Animation Init
      (bind _asbp_first_person_player (Utilities|Casting|CastToBP_FirstPersonPlayer (Pawn|GetControlledPawn (Game|GetPlayerController 0))))
      (Variables|Default|SetFirstPersonPlayer _asbp_first_person_player)
      (bind _asabp_npcbase (Utilities|Casting|CastToABP_NPCBase (Components|SkeletalMesh|GetAnimInstance (Variables|Character|GetMesh))))
      (Variables|Default|SetABP%20NPCBase _asabp_npcbase)
      (Variables|/Game/Characters/NPC/ABP_NPCBase.ABP_NPCBase_C|SetbEnableLookAt (Variables|Default|GetABP%20NPCBase) false))
    (:then_1
      ;[0.15 0.15 0.15 0.5] Dialgoue Init
      (EventDispatchers|AssignOnDialogueActiveChanged (Subsystems|GetCCDialogueSubsystem) (delegate Custom|OnDialogueActiveChanged_Event)))))

(event EventTick
  (params (DeltaSeconds :type Float%20%28single-precision%29))
  (|CallParentFunction DeltaSeconds)
  (Utilities|FlowControl|Sequence
    (:then_0
      ;[0.15 0.15 0.15 0.5] Comment
      (Variables|/Game/Characters/NPC/ABP_NPCBase.ABP_NPCBase_C|SetLookAtTarget (Variables|Default|GetABP%20NPCBase) (Transformation|GetWorldLocation (Variables|/Game/Characters/Player/BP_FirstPersonPlayer.BP_FirstPersonPlayer_C|GetLookAtTarget (Variables|Default|GetFirstPersonPlayer)))))
    (:then_1
      ;[0.15 0.15 0.15 0.5] Update ABP NPC State
      (Variables|/Game/Characters/NPC/ABP_NPCBase.ABP_NPCBase_C|SetNPCState (Variables|Default|GetABP%20NPCBase) (Class|NPCBase|GetNPCState)))))

(event EventStartChessMoveAnimation
  (params (MoveData :type Chess%20Move%20Animation%20Data%20Structure%20%28by%20ref%29))
  (Default|SetPiecePickupandPlaceLocation (Variables|Default|GetABP%20NPCBase) (.fromws MoveData) (.tows MoveData))
  (bind _notifyname (Animation|Montage|PlayMontage (Variables|Character|GetMesh) "/Game/Characters/VRMBase/Anims/AM_ChessPickupAndPlace.AM_ChessPickupAndPlace")
    (:OnCompleted
      (Class|NPCBase|FinishChessMoveAnimation (.moveid MoveData)))
    (:OnNotifyBegin
      (switch name _notifyname
        (:Pickup
          (Transformation|AttachComponentToComponent (.pieceactor MoveData) (Variables|Character|GetMesh) "ChessPieceSocket" "SnapToTarget" "SnapToTarget" "KeepRelative" true))
        (:Place
          (Class|ChessPiece|DetatchwithTween (.pieceactor MoveData) (.tows MoveData) "0, 0, 0" 0.15))))))

(fn ConstructionScript)

(fn GetInteractionName
  (return "Talk"))

(fn CanInteract
  (params (Interactor :type Pawn%20Object%20Reference))
  (return true))

(fn GetStateTree
  (bind _asbp_npc_aicontroller (Utilities|Casting|CastToBP_NPC_AIController (AI|GetAIController self)))
  (return (Variables|/Game/Characters/NPC/AI/BP_NPC_AIController.BP_NPC_AIController_C|GetStateTreeAI _asbp_npc_aicontroller)))