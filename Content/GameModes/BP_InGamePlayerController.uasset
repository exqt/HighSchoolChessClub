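; In-game player controller that sets up the gameplay UI when play begins.
; On BeginPlay it creates the primary layout widget, registers it with the CCUI subsystem, and asynchronously pushes the in-game main screen onto the InGame stack.
; It then switches input to game-only without flushing.
; A debug F key prints the player pawn's display name.
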(event EventBeginPlay
  (Utilities|FlowControl|Sequence
    (:then_0
      (bind _returnvalue (UserInterface|CreateWidget "/Game/UI/Widgets/WBP_PrimaryLayout.WBP_PrimaryLayout_C"))
      (UserInterface|Viewport|AddtoViewport _returnvalue 0)
      (Class|CCUISubsystem|RegisterCreatedPrimaryLayoutWidget (Subsystems|GetCCUISubsystem) _returnvalue))
    (:then_1
      (|PushSoftWidgettoStackAsync "(TagName=\"UI.Stack.InGame\")" "/Game/UI/Widgets/InGame/WBP_InGameMainScreen.WBP_InGameMainScreen_C"))
    (:then_2
      (Input|SetInputModeGameOnly (Game|GetPlayerController 0) false))))

(event Input|KeyboardEvents|DebugKeyF
  (params (Key :type Key%20Structure :default "None") (ActionValue :type Input%20Action%20Value%20Structure))
  (:Pressed
    (Development|PrintString (Utilities|GetDisplayName (Game|Player|GetPlayerPawn 0)))))

(fn ConstructionScript)