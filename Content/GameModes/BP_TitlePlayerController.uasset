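; Player controller for the title screen that sets up the menu UI, camera view and audio when play begins.
; It initializes the primary layout through the CCUISubsystem, switches to UI-only input focused on it, and asynchronously pushes the title screen widget onto the title stack.
; The view target becomes the first actor tagged "Camera", and a user bus mix is activated before the music plays.
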(event EventBeginPlay
  (bind _self self)
  (Utilities|FlowControl|Sequence
    (:then_0
      (bind _returnvalue (Class|CCUISubsystem|InitializePrimaryLayout (Subsystems|GetCCUISubsystem) _self))
      (Input|SetInputModeUIOnly _self _returnvalue "DoNotLock" false))
    (:then_1
      (bind _outactors (Actor|GetAllActorswithTag "Camera"))
      (Game|Player|SetViewTargetwithBlend (Utilities|Array|Get(acopy) _outactors) 0.0 "VTBlend_Linear" 0.0 false))
    (:then_2
      (|PushSoftWidgettoStackAsync "(TagName=\"UI.Stack.Title\")" "/Game/UI/Widgets/Title/WBP_TitleScreen.WBP_TitleScreen_C"))
    (:then_3
      (Class|AudioModulationStatics|ActivateBusMix "/Game/Audio/CBM_User.CBM_User")
      (Audio|SpawnSound2D "/Game/Audio/BGM/GymnopedieNo1.GymnopedieNo1" 1.0 1.0 0.0 0))))

(fn ConstructionScript)